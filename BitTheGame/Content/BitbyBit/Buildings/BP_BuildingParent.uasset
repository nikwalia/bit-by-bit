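; Base building for a turn-based strategy game, handling placement, selection and enemy spotting.
; Unplaced player buildings follow the cursor, swapping red/green materials and collision from per-tick overlap checks, then restore saved materials when clicked to place.
; Selection goes through TurnBasedController, focuses the camera and opens a build, train or upgrade menu by casting self to Farm, Castle or Forge.
; Enemy buildings use AI perception to track spotted player units and buildings.
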(event OnTargetPerceptionUpdated(AIPerception)
  (params (Actor :type Actor%20Object%20Reference) (Stimulus :type AI%20Stimulus%20Structure))
  (bind _bsuccessfullysensed (Utilities|Struct|BreakAIStimulus Stimulus))
  (bind _spottedplayerunits (Variables|Default|GetSpottedPlayerUnits))
  (bind _spottedplayerbuildings (Variables|Default|GetSpottedPlayerBuildings))
  (if (not (Variables|Default|GetPlayerOwner))
    (bind _asbase_unit (Utilities|Casting|CastToBaseUnit Actor)
      (:then
        (if (Variables|/Game/BitbyBit/Units/BaseUnit.BaseUnit_C|GetPlayerOwner _asbase_unit)
          (if _bsuccessfullysensed
            (Utilities|Set|Add _spottedplayerunits _asbase_unit)
            (else
              (Utilities|Set|Remove _spottedplayerunits _asbase_unit)))))
      (:CastFailed
        (bind _asbp_building_parent (Utilities|Casting|CastToBP_BuildingParent Actor))
        (if (Variables|BP_BuildingParent_C|GetPlayerOwner _asbp_building_parent)
          (if _bsuccessfullysensed
            (Utilities|Set|Add _spottedplayerbuildings _asbp_building_parent)
            (else
              (Utilities|Set|Remove _spottedplayerbuildings _asbp_building_parent))))))))

(event Custom|PlaceBuilding
  (CallFunction|SetMeshMaterials)
  (Variables|Default|SetIsPlaced true)
  (Rendering|Components|Light|SetIntensity (Variables|Default|GetSpotLight) 1e+07))

(event EventBeginPlay
  (bind _selectioncomponent (Variables|Components|GetSelectionComponent))
  (bind _asturn_based_controller (Utilities|Casting|CastToTurnBasedController (Game|GetPlayerController 0)))
  (Variables|Default|SetAs%20Turn%20Based%20Controller _asturn_based_controller)
  (if (Variables|Default|GetPlayerOwner)
    (Components|Tick|SetComponentTickEnabled (Variables|Default|GetAIPerception) false)
    (if (Variables|Default|GetIsPlaced)
      (Rendering|Components|Light|SetIntensity (Variables|Default|GetSpotLight) 1e+07))
    (else
      (Rendering|Components|Decal|SetDecalMaterial _selectioncomponent "/Game/BitbyBit/Textures/M_RedEnemy.M_RedEnemy")
      (Rendering|SetVisibility _selectioncomponent true false)
      (Rendering|Components|Light|SetIntensity (Variables|Default|GetSpotLight) 0.0)
      (Components|Tick|SetComponentTickEnabled (Variables|Default|GetAIPerceptionStimuliSource) false))))

(event MouseInput|EventActorOnClicked
  (params (ButtonPressed :type Key%20Structure :default "None"))
  (if (and (not (Variables|Default|GetIsPlaced)) (Variables|Default|GetPlayerOwner))
    (CallFunction|PlaceBuilding)))

(event EventTick
  (params (DeltaSeconds :type Float%20%28single-precision%29))
  (bind _overlappingactors (Collision|GetOverlappingActors "/Game/BitbyBit/Buildings/SM_BridgePiece_Blueprint.SM_BridgePiece_Blueprint_C" :!class /Script/Engine.Actor))
  (bind _overlappingactors_2 (Collision|GetOverlappingActors "BP_BuildingParent_C" :!class /Script/Engine.Actor))
  (bind _returnvalue (Game|GetPlayerController 0))
  (bind _overlappingactors_3 (Collision|GetOverlappingActors "/Game/BitbyBit/Units/BaseUnit.BaseUnit_C" :!class /Script/Engine.Actor))
  (bind _overlappingactors_4 (Collision|GetOverlappingActors "/Script/Engine.StaticMeshActor" :!class /Script/Engine.Actor))
  (bind _overlappingactors_5 (Collision|GetOverlappingActors "/Game/GreenwoodFantasyVillage/Blueprints/BP_Bonfire.BP_Bonfire_C" :!class /Script/Engine.Actor))
  (bind _overlappingactors_6 (Collision|GetOverlappingActors "/Game/GreenwoodFantasyVillage/Blueprints/BP_BonfireAssembled.BP_BonfireAssembled_C" :!class /Script/Engine.Actor))
  (bind _overlappingactors_7 (Collision|GetOverlappingActors "/Game/GreenwoodFantasyVillage/Blueprints/BP_GardenBed_Cabbage.BP_GardenBed_Cabbage_C" :!class /Script/Engine.Actor))
  (bind _overlappingactors_8 (Collision|GetOverlappingActors "/Game/GreenwoodFantasyVillage/Blueprints/BP_GardenBed_Corn.BP_GardenBed_Corn_C" :!class /Script/Engine.Actor))
  (bind _overlappingactors_9 (Collision|GetOverlappingActors "/Game/GreenwoodFantasyVillage/Blueprints/BP_GardenBed_Empty.BP_GardenBed_Empty_C" :!class /Script/Engine.Actor))
  (bind _overlappingactors_10 (Collision|GetOverlappingActors "/Game/GreenwoodFantasyVillage/Blueprints/BP_GardenBed_Onion.BP_GardenBed_Onion_C" :!class /Script/Engine.Actor))
  (bind _overlappingactors_11 (Collision|GetOverlappingActors "/Game/GreenwoodFantasyVillage/Blueprints/BP_GardenBed_Pumpkin.BP_GardenBed_Pumpkin_C" :!class /Script/Engine.Actor))
  (bind _overlappingactors_12 (Collision|GetOverlappingActors "/Game/GreenwoodFantasyVillage/Blueprints/BP_Light_cold_ON.BP_Light_cold_ON_C" :!class /Script/Engine.Actor))
  (bind _overlappingactors_13 (Collision|GetOverlappingActors "/Game/GreenwoodFantasyVillage/Blueprints/BP_Light_cold_OFF.BP_Light_cold_OFF_C" :!class /Script/Engine.Actor))
  (bind _overlappingactors_14 (Collision|GetOverlappingActors "/Game/GreenwoodFantasyVillage/Blueprints/BP_Lighthouse.BP_Lighthouse_C" :!class /Script/Engine.Actor))
  (bind _overlappingactors_15 (Collision|GetOverlappingActors "/Game/GreenwoodFantasyVillage/Blueprints/BP_LightStand_cold_ON.BP_LightStand_cold_ON_C" :!class /Script/Engine.Actor))
  (bind _overlappingactors_16 (Collision|GetOverlappingActors "/Game/GreenwoodFantasyVillage/Blueprints/BP_Mill.BP_Mill_C" :!class /Script/Engine.Actor))
  (bind _overlappingactors_17 (Collision|GetOverlappingActors "/Game/GreenwoodFantasyVillage/Blueprints/BP_LightStand_warm_ON.BP_LightStand_warm_ON_C" :!class /Script/Engine.Actor))
  (bind _overlappingactors_18 (Collision|GetOverlappingActors "/Game/GreenwoodFantasyVillage/Blueprints/BP_Light_warm_ON.BP_Light_warm_ON_C" :!class /Script/Engine.Actor))
  (bind _overlappingactors_19 (Collision|GetOverlappingActors "/Game/BitbyBit/Buildings/SM_Ground_16m_River_Water_Blueprint.SM_Ground_16m_River_Water_Blueprint_C" :!class /Script/Engine.Actor))
  (bind _returnvalue_2 (Utilities|Array|Length _overlappingactors_16))
  (bind _returnvalue_3 (Utilities|Array|Length _overlappingactors_19))
  (bind _returnvalue_4 (Utilities|Array|Length _overlappingactors_9))
  (bind _returnvalue_5 (Utilities|Array|Length _overlappingactors_10))
  (bind _returnvalue_6 (Utilities|Array|Length _overlappingactors_11))
  (bind _returnvalue_7 (Utilities|Array|Length _overlappingactors_12))
  (bind _returnvalue_8 (Utilities|Array|Length _overlappingactors_13))
  (bind _returnvalue_9 (Utilities|Array|Length _overlappingactors_14))
  (bind _returnvalue_10 (Utilities|Array|Length _overlappingactors_15))
  (bind _returnvalue_11 (Utilities|Array|Length _overlappingactors_17))
  (bind _returnvalue_12 (Utilities|Array|Length _overlappingactors_18))
  (bind _returnvalue_13 (Utilities|Array|Length _overlappingactors_2))
  (bind _returnvalue_14 (Utilities|Array|Length _overlappingactors))
  (bind _returnvalue_15 (Utilities|Array|Length _overlappingactors_3))
  (bind _returnvalue_16 (Utilities|Array|Length _overlappingactors_4))
  (bind _returnvalue_17 (Utilities|Array|Length _overlappingactors_5))
  (bind _returnvalue_18 (Utilities|Array|Length _overlappingactors_6))
  (bind _returnvalue_19 (Utilities|Array|Length _overlappingactors_7))
  (bind _returnvalue_20 (Utilities|Array|Length _overlappingactors_8))
  (bind (_hitresult _returnvalue_21) (Game|Player|GetHitResultUnderCursorbyChannel _returnvalue "TraceTypeQuery1" true))
  (bind _returnvalue_22 (== _returnvalue_13 0))
  (bind _returnvalue_23 (== _returnvalue_15 0))
  (bind _returnvalue_24 (== _returnvalue_14 0))
  (bind _location (Collision|BreakHitResult _hitresult))
  (bind _returnvalue_25 (== _returnvalue_3 0))
  (bind _returnvalue_26 (+ _returnvalue_16 _returnvalue_17 _returnvalue_18 _returnvalue_19 _returnvalue_20 _returnvalue_4 _returnvalue_5 _returnvalue_6 _returnvalue_7 _returnvalue_8 _returnvalue_9 _returnvalue_10 _returnvalue_11 _returnvalue_12 _returnvalue_2))
  (bind _returnvalue_27 (== _returnvalue_26 0))
  (bind _returnvalue_28 (Math|Boolean|ANDBoolean _returnvalue_25 _returnvalue_24 _returnvalue_22 _returnvalue_23 _returnvalue_27))
  (if (and (not (Variables|Default|GetIsPlaced)) (Variables|Default|GetPlayerOwner))
    (Utilities|FlowControl|Sequence
      (:then_0
        (if (Variables|Default|GetCollisionDisabled)
          (if _returnvalue_28
            (Utilities|FlowControl|Sequence
              (:then_0
                (goto _label_2 Reset))
              (:then_1
                (Utilities|FlowControl|DoOnce false :!label _label
                  (:Completed
                    (CallFunction|SetGreenPlacement)
                    (CallFunction|EnableCollisions)
                    (Variables|Default|SetCollisionDisabled false)
                    (Utilities|FlowControl|Delay 0.2))))))
          (elif (not _returnvalue_28)
            (Utilities|FlowControl|Sequence
              (:then_0
                (goto _label Reset))
              (:then_1
                (Utilities|FlowControl|DoOnce false :!label _label_2
                  (:Completed
                    (CallFunction|SetRedPlacement)
                    (CallFunction|DisableCollisions)
                    (Variables|Default|SetCollisionDisabled true)
                    (Utilities|FlowControl|Delay 0.2))))))))
      (:then_1
        (if _returnvalue_21
          (Transformation|SetWorldLocation (Variables|Components|GetDefaultSceneRoot) (Math|Vector|MakeVector (.x _location) (.y _location) 0.0) false false))))))

(fn ConstructionScript
  (bind _spotlight (Variables|Default|GetSpotLight))
  (if (Variables|Default|GetPlayerOwner)
    (if (Variables|Default|GetIsPlaced)
      (Rendering|Components|Light|SetIntensity _spotlight 1e+07))
    (else
      (Rendering|Components|Light|SetIntensity _spotlight 0.0))))

(fn DoSelection
  (bind _self self)
  (bind _as_turn_based_controller (Variables|Default|GetAs%20Turn%20Based%20Controller))
  (if (Variables|Default|GetPlayerOwner)
    (bind _asturn_based_controller (Utilities|Casting|CastToTurnBasedController (Game|GetPlayerController 0)))
    (Default|SelectBuilding _asturn_based_controller self)
    (if (Variables|Default|GetSelected)
      (Rendering|SetVisibility (Variables|Components|GetSelectionComponent) true false)
      (if (Utilities|IsValid _as_turn_based_controller)
        (Default|SetCameraLocation _as_turn_based_controller (Transformation|GetActorLocation)))
      ;[1 1 1] Handle different menus for different buildings
      (Utilities|Casting|CastToBP_Farm _self
        (:then
          (bind _returnvalue (UserInterface|CreateWidget "/Game/BitbyBit/Buildings/BuildingUI/UIBuildBaseMenu.UIBuildBaseMenu_C"))
          (bind _output_get (Variables|Default|SetBuildMenu _returnvalue))
          (UserInterface|Viewport|AddtoViewport _output_get 0)
          (Variables|/Game/BitbyBit/TurnBasedController.TurnBasedController_C|SetIsZoomEnabled (Variables|Default|GetAs%20Turn%20Based%20Controller) false))
        (:CastFailed
          (Utilities|Casting|CastToBP_Castle _self
            (:then
              (bind _returnvalue_2 (UserInterface|CreateWidget "/Game/BitbyBit/Buildings/BuildingUI/UITrainBaseMenu.UITrainBaseMenu_C"))
              (bind _output_get_2 (Variables|Default|SetTrainMenu _returnvalue_2))
              (UserInterface|Viewport|AddtoViewport _output_get_2 0)
              (Variables|/Game/BitbyBit/TurnBasedController.TurnBasedController_C|SetIsZoomEnabled (Variables|Default|GetAs%20Turn%20Based%20Controller) false))
            (:CastFailed
              (Utilities|Casting|CastToBP_Forge _self)
              (bind _returnvalue_3 (UserInterface|CreateWidget "/Game/BitbyBit/Buildings/BuildingUI/UIUpgradeBaseMenu.UIUpgradeBaseMenu_C"))
              (bind _output_get_3 (Variables|Default|SetUpgradeMenu _returnvalue_3))
              (UserInterface|Viewport|AddtoViewport _output_get_3 0)
              (Variables|/Game/BitbyBit/TurnBasedController.TurnBasedController_C|SetIsZoomEnabled (Variables|Default|GetAs%20Turn%20Based%20Controller) false)))))
      (else
        (Rendering|SetVisibility (Variables|Components|GetSelectionComponent) false false)
        (if (Utilities|IsValid (Variables|Default|GetBuildMenu))
          (Widget|RemovefromParent (Variables|Default|GetBuildMenu))
          (Variables|Default|SetBuildMenu 0)
          (Variables|Default|SetTrainMenu 0)
          (Variables|Default|SetUpgradeMenu 0))))))

(fn SetGreenPlacement
  (bind _savedmaterials (Variables|Default|GetSavedMaterials))
  (bind _keys (Utilities|Map|Keys (Variables|Default|GetMeshMap)))
  (for (_array_element _array_index) _keys
    (for (_array_element_2 _array_index_2) (Rendering|Material|GetMaterials _array_element)
      (if (== (Utilities|Map|Length _savedmaterials) 0)
        (Utilities|Map|Add _savedmaterials (Math|Conversions|ToInteger(Byte) (Utilities|String|Append (Utilities|String|ToString(Integer) _array_index) (Utilities|String|ToString(Integer) _array_index_2))) _array_element_2))
      (Rendering|Material|SetMaterial _array_element _array_index_2 "/Game/BitbyBit/Textures/T_GreenPlacement.T_GreenPlacement"))
    (Variables|Default|SetIsPlaced false)))

(fn SetMeshMaterials
  (bind _keys (Utilities|Map|Keys (Variables|Default|GetMeshMap)))
  (for (_array_element _array_index) _keys
    (for (_ _array_index_2) (Rendering|Material|GetMaterials _array_element)
      (Rendering|Material|SetMaterial _array_element _array_index_2 (.Value (Utilities|Map|Find (Variables|Default|GetSavedMaterials) (Math|Conversions|ToInteger(Byte) (Utilities|String|Append (Utilities|String|ToString(Integer) _array_index) (Utilities|String|ToString(Integer) _array_index_2)))))))))

(fn SetRedPlacement
  (bind _savedmaterials (Variables|Default|GetSavedMaterials))
  (bind _keys (Utilities|Map|Keys (Variables|Default|GetMeshMap)))
  (for (_array_element _array_index) _keys
    (for (_array_element_2 _array_index_2) (Rendering|Material|GetMaterials _array_element)
      (if (== (Utilities|Map|Length _savedmaterials) 0)
        (Utilities|Map|Add _savedmaterials (Math|Conversions|ToInteger(Byte) (Utilities|String|Append (Utilities|String|ToString(Integer) _array_index) (Utilities|String|ToString(Integer) _array_index_2))) _array_element_2))
      (Rendering|Material|SetMaterial _array_element _array_index_2 "/Game/BitbyBit/Textures/T_RedPlacement.T_RedPlacement"))
    (Variables|Default|SetIsPlaced false)))

(fn DisableCollisions
  (for _array_element (Variables|Default|GetBoxChildren)
    (Utilities|IsValid _array_element
      (:Is%20Valid
        (Utilities|Casting|CastToStaticMeshComponent _array_element
          (:then
            _)
          (:CastFailed
            (Utilities|Casting|CastToDestructibleComponent _array_element)))
        (bind _asprimitive_component (Utilities|Casting|CastToPrimitiveComponent _array_element))
        (Collision|SetCollisionResponsetoAllChannels _asprimitive_component "ECR_Ignore"))))
  (for _array_element_2 (Variables|Default|GetBlockboxes)
    (Collision|SetCollisionResponsetoAllChannels _array_element_2 "ECR_Ignore")))

(fn EnableCollisions
  (for _array_element (Variables|Default|GetBoxChildren)
    (Utilities|IsValid _array_element
      (:Is%20Valid
        (Utilities|Casting|CastToStaticMeshComponent _array_element
          (:then
            _)
          (:CastFailed
            (Utilities|Casting|CastToDestructibleComponent _array_element)))
        (bind _asprimitive_component (Utilities|Casting|CastToPrimitiveComponent _array_element))
        (Collision|SetCollisionResponsetoChannel _asprimitive_component "ECC_Visibility" "ECR_Overlap"))))
  (for _array_element_2 (Variables|Default|GetBlockboxes)
    (Collision|SetCollisionResponsetoAllChannels _array_element_2 "ECR_Block"))
  (for _array_element_3 (Variables|Default|GetClickboxes)
    (Collision|SetCollisionResponsetoAllChannels _array_element_3 "ECR_Block")))

(fn HandleAttackfromUnits
  (bind _asturn_based_controller (Utilities|Casting|CastToTurnBasedController (Game|GetPlayerController 0))))

(fn HandleDestroyed
  (if (Variables|Default|GetPlayerOwner)
    (bind _asturn_based_game_mode (Utilities|Casting|CastToTurnBasedGameMode (Game|GetGameMode)))
    (Default|DeleteBuilding _asturn_based_game_mode self)))