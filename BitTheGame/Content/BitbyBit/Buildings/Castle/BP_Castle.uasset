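; Castle building for a turn-based game, made of a town hall and a lighthouse that take damage and collapse independently.
; Construction registers block and click boxes with inherited arrays and maps each mesh to its damage function by name; left-clicks trigger selection.
; Damage applies only once placed and ends the controller's attack.
; Tick polls both healths, dropping depleted parts with physics before removing them, and destroys the actor when both are gone.
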(event OnClicked(LighthouseClickBox)
  (params (TouchedComponent :type Primitive%20Component%20Object%20Reference) (ButtonPressed :type Key%20Structure :default "None"))
  (if (== "LeftMouseButton" ButtonPressed)
    (CallFunction|DoSelection)))

(event OnClicked(TownHallClickbox)
  (params (TouchedComponent :type Primitive%20Component%20Object%20Reference) (ButtonPressed :type Key%20Structure :default "None"))
  (if (== "LeftMouseButton" ButtonPressed)
    (CallFunction|DoSelection)))

(event Custom|DestroyLighthouse
  (Physics|SetSimulatePhysics (Variables|Default|GetLighthouse) true)
  (Components|DestroyComponent (Variables|Default|GetLighthouseBlockBox))
  (Components|DestroyComponent (Variables|Default|GetLighthouseHitBox))
  (Utilities|FlowControl|Delay 2.5)
  (Components|DestroyComponent (Variables|Default|GetLighthouse)))

(event Custom|DestroyBuilding
  (Physics|SetSimulatePhysics (Variables|Default|GetTownHall) true)
  (Physics|SetSimulatePhysics (Variables|Default|GetTownHall1) true)
  (Components|DestroyComponent (Variables|Default|GetTownHallBlockbox))
  (Components|DestroyComponent (Variables|Default|GetTownHallHitbox))
  (Utilities|FlowControl|Delay 2.5)
  (Components|DestroyComponent (Variables|Default|GetTownHall))
  (Components|DestroyComponent (Variables|Default|GetTownHall1)))

(event EventBeginPlay
  (|CallParentFunction))

(event EventTick
  (params (DeltaSeconds :type Float%20%28single-precision%29))
  (bind _buildinghealth (Variables|Default|GetBuildingHealth))
  (bind _lighthousehealth (Variables|Default|GetLighthouseHealth))
  (bind _returnvalue (< _buildinghealth 0.1))
  (bind _returnvalue_2 (< _lighthousehealth 0.1))
  (|CallParentFunction 0.0)
  (Utilities|FlowControl|Sequence
    (:then_0
      (if _returnvalue
        (Utilities|FlowControl|Delay 1.0)
        (CallFunction|DestroyBuilding)))
    (:then_1
      (if _returnvalue_2
        (Utilities|FlowControl|Delay 1.0)
        (CallFunction|DestroyLighthouse)))
    (:then_2
      (if (and _returnvalue _returnvalue_2)
        (Utilities|FlowControl|Delay 2.5)
        (CallFunction|HandleDestroyed)
        (Actor|DestroyActor)))))

(fn ConstructionScript
  (bind _blockboxes (Variables|Default|GetBlockboxes))
  (bind _clickboxes (Variables|Default|GetClickboxes))
  (Variables|Default|SetSelectionComponent (Variables|Default|GetSelection))
  (Utilities|Array|Add _blockboxes (Variables|Default|GetLighthouseBlockBox))
  (Utilities|Array|Add _blockboxes (Variables|Default|GetTownHallBlockbox))
  (Variables|Default|SetBoxChildren (Components|GetChildrenComponents (Variables|Default|GetBox) true))
  (Utilities|Array|Add _clickboxes (Variables|Default|GetTownHallClickbox))
  (Utilities|Array|Add _clickboxes (Variables|Default|GetLighthouseClickBox))
  (Variables|Default|SetMeshMap (Utilities|Map|MakeMap (Variables|Default|GetLighthouse) (Utilities|Name|MakeLiteralName "TakeLighthouseDamage") (Variables|Default|GetTownHall1) (Utilities|Name|MakeLiteralName "TakeBuildingDamage") (Variables|Default|GetTownHall) (Utilities|Name|MakeLiteralName "TakeBuildingDamage"))))

(fn TakeBuildingDamage
  (if (Variables|Default|GetIsPlaced)
    (Variables|Default|SetBuildingHealth (- (Variables|Default|GetBuildingHealth) (Variables|Default|GetLatestDamage)))
    (bind _asturn_based_controller (Utilities|Casting|CastToTurnBasedController (Game|GetPlayerController 0)))
    (Default|FinishAttack _asturn_based_controller)))

(fn TakeLighthouseDamage
  (if (Variables|Default|GetIsPlaced)
    (Variables|Default|SetLighthouseHealth (- (Variables|Default|GetLighthouseHealth) (Variables|Default|GetLatestDamage)))
    (bind _asturn_based_controller (Utilities|Casting|CastToTurnBasedController (Game|GetPlayerController 0)))
    (Default|FinishAttack _asturn_based_controller)))