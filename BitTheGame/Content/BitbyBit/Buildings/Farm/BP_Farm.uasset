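; Farm building with three destructible parts (main building, wagon and well), selectable by left-clicking any part.
; Once placed, each part loses health when a BaseUnit overlaps its hitbox, then collapses with physics and is removed after a delay.
; Tick destroys the actor when all three are depleted.
; The construction script registers components in arrays for blockboxes, clickboxes and meshes; pumpkin and corn bed spawning is unconnected.
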(event OnComponentBeginOverlap(WagonHitbox)
  (params (OverlappedComponent :type Primitive%20Component%20Object%20Reference) (OtherActor :type Actor%20Object%20Reference) (OtherComp :type Primitive%20Component%20Object%20Reference) (OtherBodyIndex :type Integer) (bFromSweep :type Boolean) (SweepResult :type Hit%20Result%20Structure%20%28by%20ref%29))
  (if (Variables|Default|GetIsPlaced)
    (bind _asbase_unit (Utilities|Casting|CastToBaseUnit OtherActor))
    (bind _output_get (Variables|Default|SetWagonHealth (- (Variables|Default|GetWagonHealth) (Variables|/Game/BitbyBit/Units/BaseUnit.BaseUnit_C|GetDamage _asbase_unit))))
    (if (< _output_get 0.1)
      (Physics|SetSimulatePhysics (Variables|Default|GetWheelbarrow) true)
      (Components|DestroyComponent (Variables|Default|GetWagonBlockbox))
      (Components|DestroyComponent (Variables|Default|GetWagonHitbox))
      (Utilities|FlowControl|Delay 2.5)
      (Components|DestroyComponent (Variables|Default|GetWheelbarrow)))))

(event OnComponentBeginOverlap(WellHitbox)
  (params (OverlappedComponent :type Primitive%20Component%20Object%20Reference) (OtherActor :type Actor%20Object%20Reference) (OtherComp :type Primitive%20Component%20Object%20Reference) (OtherBodyIndex :type Integer) (bFromSweep :type Boolean) (SweepResult :type Hit%20Result%20Structure%20%28by%20ref%29))
  (if (Variables|Default|GetIsPlaced)
    (bind _asbase_unit (Utilities|Casting|CastToBaseUnit OtherActor))
    (bind _output_get (Variables|Default|SetWellHealth (- (Variables|Default|GetWellHealth) (Variables|/Game/BitbyBit/Units/BaseUnit.BaseUnit_C|GetDamage _asbase_unit))))
    (if (< _output_get 0.1)
      (Physics|SetSimulatePhysics (Variables|Default|GetWell) true)
      (Components|DestroyComponent (Variables|Default|GetWellBlockbox))
      (Components|DestroyComponent (Variables|Default|GetWellHitbox))
      (Utilities|FlowControl|Delay 2.5)
      (Components|DestroyComponent (Variables|Default|GetWell)))))

(event OnClicked(BuildingClickBox)
  (params (TouchedComponent :type Primitive%20Component%20Object%20Reference) (ButtonPressed :type Key%20Structure :default "None"))
  (if (== "LeftMouseButton" ButtonPressed)
    (CallFunction|DoSelection)))

(event OnClicked(WagonClickBox)
  (params (TouchedComponent :type Primitive%20Component%20Object%20Reference) (ButtonPressed :type Key%20Structure :default "None"))
  (if (== ButtonPressed "LeftMouseButton")
    (CallFunction|DoSelection)))

(event OnClicked(WellClickBox)
  (params (TouchedComponent :type Primitive%20Component%20Object%20Reference) (ButtonPressed :type Key%20Structure :default "None"))
  (if (== ButtonPressed "LeftMouseButton")
    (CallFunction|DoSelection)))

(event OnComponentBeginOverlap(BuildingHitbox)
  (params (OverlappedComponent :type Primitive%20Component%20Object%20Reference) (OtherActor :type Actor%20Object%20Reference) (OtherComp :type Primitive%20Component%20Object%20Reference) (OtherBodyIndex :type Integer) (bFromSweep :type Boolean) (SweepResult :type Hit%20Result%20Structure%20%28by%20ref%29))
  (if (Variables|Default|GetIsPlaced)
    (bind _asbase_unit (Utilities|Casting|CastToBaseUnit OtherActor))
    (bind _output_get (Variables|Default|SetBuildingHealth (- (Variables|Default|GetBuildingHealth) (Variables|/Game/BitbyBit/Units/BaseUnit.BaseUnit_C|GetDamage _asbase_unit))))
    (if (< _output_get 0.1)
      (Physics|SetSimulatePhysics (Variables|Default|GetBuilding) true)
      (Components|DestroyComponent (Variables|Default|GetBuildingBlockbox))
      (Components|DestroyComponent (Variables|Default|GetBuildingHitbox))
      (Utilities|FlowControl|Delay 2.5)
      (Components|DestroyComponent (Variables|Default|GetBuilding)))))

(event EventBeginPlay
  (|CallParentFunction))

(event EventTick
  (params (DeltaSeconds :type Float%20%28single-precision%29))
  (|CallParentFunction 0.0)
  (if (Math|Boolean|ANDBoolean (< (Variables|Default|GetBuildingHealth) 0.1) (< (Variables|Default|GetWagonHealth) 0.1) (< (Variables|Default|GetWellHealth) 0.1))
    (Utilities|FlowControl|Delay 2.5)
    (Actor|DestroyActor)))

(fn ConstructionScript
  (bind _blockboxes (Variables|Default|GetBlockboxes))
  (bind _meshes (Variables|Default|GetMeshes))
  (bind _clickboxes (Variables|Default|GetClickboxes))
  (Variables|Default|SetSelectionComponent (Variables|Default|GetSelection))
  (Utilities|Array|Add _blockboxes (Variables|Default|GetBuildingBlockbox))
  (Utilities|Array|Add _blockboxes (Variables|Default|GetWagonBlockbox))
  (Utilities|Array|Add _blockboxes (Variables|Default|GetWellBlockbox))
  (Variables|Default|SetBoxChildren (Components|GetChildrenComponents (Variables|Default|GetBox) true))
  (Utilities|Array|Add _clickboxes (Variables|Default|GetBuildingClickBox))
  (Utilities|Array|Add _clickboxes (Variables|Default|GetWagonClickBox))
  (Utilities|Array|Add _clickboxes (Variables|Default|GetWellClickBox))
  (Utilities|Array|Add _meshes (Variables|Default|GetBuilding))
  (Utilities|Array|Add _meshes (Variables|Default|GetWheelbarrow))
  (Utilities|Array|Add _meshes (Variables|Default|GetWell)))