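; Forge building with two separately destructible parts, the main building and a trough, both left-clickable for selection.
; Overlapping fighters subtract their Damage from that part's health; a depleted part drops with physics, loses its collision and is removed after a delay.
; Tick destroys the actor once both parts are depleted, otherwise registers it once for AI Sight and Team senses when VisibleToEnemy0 is set.
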(event OnComponentBeginOverlap(BuildingHitbox)
  (params (OverlappedComponent :type Primitive%20Component%20Object%20Reference) (OtherActor :type Actor%20Object%20Reference) (OtherComp :type Primitive%20Component%20Object%20Reference) (OtherBodyIndex :type Integer) (bFromSweep :type Boolean) (SweepResult :type Hit%20Result%20Structure%20%28by%20ref%29))
  (bind _asbp_fighter_parent (Utilities|Casting|CastToBP_FighterParent OtherActor))
  (bind _output_get (Variables|Default|SetBuildingHealth (- (Variables|Default|GetBuildingHealth) (Variables|/Game/BitbyBit/Blueprints/BP_FighterParent.BP_FighterParent_C|GetDamage _asbp_fighter_parent))))
  (if (< _output_get 0.1)
    (Physics|SetSimulatePhysics (Variables|Default|GetBuilding) true)
    (Components|DestroyComponent (Variables|Default|GetBuildingBlockbox))
    (Components|DestroyComponent (Variables|Default|GetBuildingHitbox))
    (Utilities|FlowControl|Delay 2.5)
    (Components|DestroyComponent (Variables|Default|GetBuilding))))

(event OnComponentBeginOverlap(TroughHitbox)
  (params (OverlappedComponent :type Primitive%20Component%20Object%20Reference) (OtherActor :type Actor%20Object%20Reference) (OtherComp :type Primitive%20Component%20Object%20Reference) (OtherBodyIndex :type Integer) (bFromSweep :type Boolean) (SweepResult :type Hit%20Result%20Structure%20%28by%20ref%29))
  (bind _asbp_fighter_parent (Utilities|Casting|CastToBP_FighterParent OtherActor))
  (bind _output_get (Variables|Default|SetTroughHealth (- (Variables|Default|GetTroughHealth) (Variables|/Game/BitbyBit/Blueprints/BP_FighterParent.BP_FighterParent_C|GetDamage _asbp_fighter_parent))))
  (if (< _output_get 0.1)
    (Physics|SetSimulatePhysics (Variables|Default|GetTrough) true)
    (Components|DestroyComponent (Variables|Default|GetTroughBlockbox))
    (Components|DestroyComponent (Variables|Default|GetTroughHitbox))
    (Utilities|FlowControl|Delay 2.5)
    (Components|DestroyComponent (Variables|Default|GetTrough))))

(event OnClicked(BuildingClickBox)
  (params (TouchedComponent :type Primitive%20Component%20Object%20Reference) (ButtonPressed :type Key%20Structure :default "None"))
  (if (== ButtonPressed "LeftMouseButton")
    (CallFunction|DoSelection)))

(event OnClicked(TroughClickBox)
  (params (TouchedComponent :type Primitive%20Component%20Object%20Reference) (ButtonPressed :type Key%20Structure :default "None"))
  (if (== "LeftMouseButton" ButtonPressed)
    (CallFunction|DoSelection)))

(event EventTick
  (params (DeltaSeconds :type Float%20%28single-precision%29))
  (if (and (< (Variables|Default|GetBuildingHealth) 0.1) (< (Variables|Default|GetTroughHealth) 0.1))
    (Utilities|FlowControl|Delay 2.5)
    (Actor|DestroyActor)
    (elif (Variables|Default|GetVisibleToEnemy_0)
      (Utilities|FlowControl|DoOnce false
        (:Completed
          (bind _returnvalue (AddComponent|AddAIPerceptionStimuliSourceComponent))
          (Class|AIPerceptionStimuliSourceComponent|RegisterforSense _returnvalue "/Script/AIModule.AISense_Team")
          (Class|AIPerceptionStimuliSourceComponent|RegisterforSense _returnvalue "/Script/AIModule.AISense_Sight"))))))

(fn ConstructionScript
  (Variables|Default|SetSelectionComponent (Variables|Default|GetSelection)))